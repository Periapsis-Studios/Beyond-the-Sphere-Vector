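; BP_AstronomicalBody is an actor that simulates N-body, gravity-style motion between astronomical bodies.
; Each tick, non-static bodies loop over BP_GameData's Bodies, adding CalculateGravity's result to Velocity and moving once per other body.
; The term scales mass over squared distance by a constant and the unnormalized offset, so it falls off as 1/distance.
; As wired, it points away from the other body and ignores delta time, which scales only movement.
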(event `self.ReceiveBeginPlay`
  (bind _returnvalue (`GameplayStatics.GetActorOfClass` "/Game/Blueprints/BP_GameData.BP_GameData_C"))
  (set `self.GameController` _returnvalue))

(event `self.ReceiveTick`
  (params (DeltaSeconds :type "Float (single-precision)"))
  (bind _returnvalue (`self.K2_GetActorLocation`))
  ;[1 1 1] Gravity
  (if (not (`self.IsStatic`))
    (for _array_element (`/Game/Blueprints/BP_GameData.Bodies` (`self.GameController`))
      (if (not (== self _array_element))
        (bind _asbp_astronomical_body (cast `/Game/Blueprints/BP_AstronomicalBody` _array_element))
        (bind _returnvalue_2 (`self.K2_GetActorLocation` _array_element))
        (bind _forcevector (`self.CalculateGravity` (`/Game/Blueprints/BP_AstronomicalBody.Mass` _asbp_astronomical_body) (`KismetMathLibrary.Vector_Distance` _returnvalue_2 _returnvalue) _returnvalue_2 _returnvalue))
        (bind _output_get (set `self.Velocity` (+ _forcevector (`self.Velocity`))))
        (`self.K2_AddActorWorldOffset` (* _output_get DeltaSeconds))))))

(fn `CalculateGravity`
  (params (MassOther :type "Float (double-precision)") (Distance :type "Float (double-precision)") (PositionSelf :type "Vector Structure") (PositionOther :type "Vector Structure"))
  (returns (ForceVector :type "Vector Structure"))
  (return (* (* (/ MassOther (`KismetMathLibrary.MultiplyMultiply_FloatFloat` Distance 2.0)) 990.145) (- PositionOther PositionSelf))))

(fn `UserConstructionScript`)
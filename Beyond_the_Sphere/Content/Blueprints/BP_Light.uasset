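; BP_Light is an actor that makes a directional light act like a point source at the world origin, as seen from the camera.
; On BeginPlay it caches the level's CameraActor.
; Each Tick it aims its forward axis along the origin-to-camera vector and sets intensity to Candelas divided by the squared distance, giving inverse-square falloff with a directional light.
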(event `self.ReceiveBeginPlay`
  (bind _returnvalue (`GameplayStatics.GetActorOfClass` "/Script/Engine.CameraActor"))
  (set `self.Camera` _returnvalue))

(event `self.ReceiveTick`
  (params (DeltaSeconds :type "Float (single-precision)"))
  (bind _returnvalue (`self.K2_GetActorLocation` (`self.Camera`)))
  (`self.K2_SetActorRotation` (`KismetMathLibrary.Conv_VectorToRotator` _returnvalue))
  (`LightComponent.SetIntensity` (`self.DirectionalLight`) (/ (`self.Candelas`) (`KismetMathLibrary.Vector_DistanceSquared` _returnvalue))))

(fn `UserConstructionScript`)